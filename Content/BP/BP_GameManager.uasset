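; BP_GameManager runs a Breakout level, tracking blocks, remaining balls, and clear or game-over state.
; Block counters trigger the clear widget at zero remaining, while a miss with no balls left shows game over.
; A single Action function spawns a ball, reloads the level or opens the next, depending on state.
; BeginPlay loads the ball count from BP_BreakoutGameInstance if valid, and advancing levels adds one ball.
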(event EventBeginPlay
  (bind _asbp_breakout_game_instance (Utilities|Casting|CastToBP_BreakoutGameInstance (Game|GetGameInstance)))
  (bind _isvalidballnum (Default|IsValidBallNum _asbp_breakout_game_instance))
  (if _isvalidballnum
    (Variables|Default|SetleftBallNum (Variables|/Game/BP/BP_BreakoutGameInstance.BP_BreakoutGameInstance_C|GetleftBallNum _asbp_breakout_game_instance))))

(event Collision|EventActorBeginOverlap
  (params (OtherActor :type Actor%20Object%20Reference)))

(event EventTick
  (params (DeltaSeconds :type Float%20%28single-precision%29)))

(fn ConstructionScript)

(fn AddBlockNum
  (bind _result (Math|Integer|IncrementInt (Variables|Default|GetblockNum))
    (:%20%20
      (Development|PrintString (Utilities|String|Append "AddBlockNum: " (Utilities|String|ToString(Integer) _result))))))

(fn AddBrokenBlockNum
  (bind _result (Math|Integer|IncrementInt (Variables|Default|GetbrokenBlockNum))
    (:%20%20
      (Development|PrintString (Utilities|String|Append "BrokenBlockNum: " (Utilities|String|ToString(Integer) _result)) true true "(R=0.000000,G=0.165369,B=1.000000,A=1.000000)")
      (bind _leftblocknum (CallFunction|GetLeftBlockNum))
      (Development|PrintString (Utilities|String|Append "LeftBlockNum: " (Utilities|String|ToString(Integer) _leftblocknum)) true true "(R=0.827410,G=0.000000,B=1.000000,A=1.000000)")
      (bind _leftblocknum_2 (CallFunction|GetLeftBlockNum))
      (if (== _leftblocknum_2 0)
        (CallFunction|ViewClearWIdget)
        (Variables|Default|SetIsCleard true)))))

(fn GetLeftBlockNum
  (return (- (Variables|Default|GetblockNum) (Variables|Default|GetbrokenBlockNum))))

(fn ViewClearWIdget
  (bind _returnvalue (UserInterface|CreateWidget "/Game/BP/WG_ClearWidget.WG_ClearWidget_C"))
  (UserInterface|Viewport|AddtoViewport _returnvalue 0))

(fn ViewGameOverWidget
  (bind _returnvalue (UserInterface|CreateWidget "/Game/BP/WG_GameoverWidget.WG_GameoverWidget_C"))
  (UserInterface|Viewport|AddtoViewport _returnvalue 0))

(fn MissCount
  (Variables|Default|SetisBallSpawned false)
  (if (and (<= (Variables|Default|GetleftBallNum) 0) (not (Variables|Default|GetIsCleard)))
    (CallFunction|ViewGameOverWidget)
    (Variables|Default|SetisGameOver true)))

(fn SpawnBall
  (if (and (> (Variables|Default|GetleftBallNum) 0) (not (Variables|Default|GetisBallSpawned)))
    (Game|SpawnActorfromClass "/Game/BP/BP_Ball.BP_Ball_C" (Math|Transform|MakeTransform (Transformation|GetActorLocation (Variables|Default|GetspawnLocationActor))) "Undefined" "MultiplyWithRoot" 0 0)
    (Variables|Default|SetisBallSpawned true)
    (Math|Integer|DecrementInt (Variables|Default|GetleftBallNum))))

(fn Action
  (if (Variables|Default|GetisGameOver)
    (CallFunction|LevelReset)
    (elif (Variables|Default|GetIsCleard)
      (CallFunction|OpenNextLevel)
      (else
        (CallFunction|SpawnBall)))))

(fn GetLeftBallNum
  (return (Variables|Default|GetleftBallNum)))

(fn LevelReset
  (bind _returnvalue (Game|GetCurrentLevelName true))
  (Game|OpenLevel(byName) (Utilities|String|StringToName _returnvalue)))

(fn OpenNextLevel
  (Utilities|Casting|CastToBP_BreakoutGameInstance (Game|GetGameInstance))
  (Variables|Default|SetleftBallNum (+ (Variables|Default|GetleftBallNum) 1))
  (Game|OpenLevel(byName) (Variables|Default|GetnextLevelName)))