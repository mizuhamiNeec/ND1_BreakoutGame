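; Player-controlled paddle that slides along the right vector with swept movement.
; Enhanced Input drives movement and forwards the action press to BP_GameManager, which it finds at BeginPlay.
; GetTopNormal fakes a curved top by tilting upward hit normals by the hit's Y offset from the bounds center, scaled up to MaxTiltNormalDeg.
; Tick draws debug arrows of those tilted normals across the top surface.
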(event Input|EnhancedActionEvents|EnhancedInputActionIA_Move
  (params (ActionValue :type Float%20%28double-precision%29) (ElapsedSeconds :type Float%20%28double-precision%29) (TriggeredSeconds :type Float%20%28double-precision%29) (InputAction :type Input%20Action%20Object%20Reference :default "/Game/Inputs/IA_Move.IA_Move"))
  (Transformation|SetActorLocation (+ (* (Class|KismetMathLibrary|VectorRight) ActionValue (Variables|Default|Getspeed) (Utilities|Time|GetWorldDeltaSeconds)) (Transformation|GetActorLocation)) true false))

(event Input|EnhancedActionEvents|EnhancedInputActionIA_Action
  (params (ActionValue :type Boolean) (ElapsedSeconds :type Float%20%28double-precision%29) (TriggeredSeconds :type Float%20%28double-precision%29) (InputAction :type Input%20Action%20Object%20Reference :default "/Game/Inputs/IA_Action.IA_Action"))
  (:Started
    (Default|Action (Variables|Default|GetGameManager))))

(event EventTick
  (params (DeltaSeconds :type Float%20%28single-precision%29))
  (CallFunction|DrawDebugTopSurfaceNormals))

(event EventBeginPlay
  (Input|AddMappingContext (PlayerController|LocalPlayerSubsystems|GetEnhancedInputLocalPlayerSubsystem (Game|GetPlayerController 0)) "/Game/Inputs/IMC_InGame.IMC_InGame" 0 "(bIgnoreAllPressedKeysUntilRelease=True,bForceImmediately=False,bNotifyUserSettings=False)")
  (bind _returnvalue (Actor|GetActorOfClass "/Game/BP/BP_GameManager.BP_GameManager_C"))
  (Variables|Default|SetGameManager _returnvalue))

(fn ConstructionScript)

(fn GetTopNormal
  (params (hitLocation :type Vector) (normal :type Vector))
  (bind (_origin _boxextent) (Collision|GetActorBounds false false))
  (if (Class|KismetMathLibrary|NotEqualExactlyVectorVector normal (Math|Vector|VectorUp))
    (return false normal)
    (else
      (return true (Math|Vector|RotateVector normal (Math|Rotator|MakeRotator (* (/ (- (.Y (Math|Vector|BreakVector hitLocation)) (.y _origin)) (.y _boxextent)) (Variables|Default|GetmaxTiltNormalDeg)) 0.0 0.0))))))

(fn DrawDebugArrow
  (params (Origin :type Vector) (Direction :type Vector))
  (LocalVariables|SetmShapedDirection (* (Math|Vector|Normalize Direction) (LocalVariables|GetmLength)))
  (Rendering|Debug|DrawDebugArrow Origin (+ Origin (LocalVariables|GetmShapedDirection)) 1e+02 "(R=0.000000,G=0.054052,B=1.000000,A=1.000000)" 0.0 1e+01))

(fn DrawDebugTopSurfaceNormals
  (bind (_origin _boxextent) (Collision|GetActorBounds false false))
  (bind _mdrawnumhalf (LocalVariables|GetmDrawNumHalf))
  (for _index (range (* _mdrawnumhalf -1) _mdrawnumhalf)
    (bind _outnormal (CallFunction|GetTopNormal (+ (Math|Vector|MakeVector 0.0 (* (/ (.y _boxextent) (LocalVariables|GetmDrawNumHalf)) _index) (.z _boxextent)) _origin) (Math|Vector|VectorUp)))
    (CallFunction|DrawDebugArrow (+ (Math|Vector|MakeVector 0.0 (* (/ (.y _boxextent) (LocalVariables|GetmDrawNumHalf)) _index) (.z _boxextent)) _origin) _outnormal)))