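; BP_Ball is a ball actor that travels at constant speed and bounces off what it hits.
; Each Tick moves it along its normalized Direction with a swept SetActorLocation, and Hit events mirror Direction around the surface normal.
; When its Sphere begins overlapping a component tagged MissArea, it calls MissCount on BP_GameManager and destroys itself.
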(event OnComponentBeginOverlap(Sphere)
  (params (OverlappedComponent :type Primitive%20Component%20Object%20Reference) (OtherActor :type Actor%20Object%20Reference) (OtherComp :type Primitive%20Component%20Object%20Reference) (OtherBodyIndex :type Integer) (bFromSweep :type Boolean) (SweepResult :type Hit%20Result%20Structure%20%28by%20ref%29))
  (if (Components|ComponentHasTag OtherComp "MissArea")
    (bind _returnvalue (Actor|GetActorOfClass "/Game/BP/BP_GameManager.BP_GameManager_C"))
    (Default|MissCount _returnvalue)
    (Actor|DestroyActor)))

(event EventTick
  (params (DeltaSeconds :type Float%20%28single-precision%29))
  (Transformation|SetActorLocation (+ (Transformation|GetActorLocation) (* (Math|Vector|Normalize (Variables|Default|Getdirection)) (Variables|Default|Getspeed) DeltaSeconds)) true false))

(event Collision|EventHit
  (params (MyComp :type Primitive%20Component%20Object%20Reference) (Other :type Actor%20Object%20Reference) (OtherComp :type Primitive%20Component%20Object%20Reference) (bSelfMoved :type Boolean) (HitLocation :type Vector :default "0, 0, 0") (HitNormal :type Vector :default "0, 0, 0") (NormalImpulse :type Vector :default "0, 0, 0") (Hit :type Hit%20Result%20Structure%20%28by%20ref%29))
  (Variables|Default|Setdirection (Math|Vector|MirrorVectorbyNormal (Variables|Default|Getdirection) HitNormal)))

(fn ConstructionScript)